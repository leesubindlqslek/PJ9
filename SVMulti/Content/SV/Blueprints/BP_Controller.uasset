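; BP_Controller is a controller Blueprint for multiplayer chat that links the chat window to BP_ChatMode.
; A login event stores the user ID and fires the OnUserLogin dispatcher.
; After a short BeginPlay delay on networked instances, it binds an event to Widget_ChatWindow.
; Outgoing messages reach the game mode prefixed with the user ID, while received broadcasts print to screen only with authority.
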(event `OnLoginWithID`
  (params (UserId :type String :default "UserId"))
  ; 코멘트
  (`self.OnUserLogin` UserId)
  (set `self.Userld` UserId))

(event `GotBroadcast`
  (params (Msg :type String :default "Msg"))
  ; 코멘트
  (if (`self.HasAuthority`)
    (`KismetSystemLibrary.PrintString` Msg true true (struct :`G` 0.66 :`B` 1.0 :`A` 1.0) 10.0)))

(event `OnSendMsgToServer`
  (params (Msg :type String))
  ; 코멘트
  (bind _asbp_chat_mode (cast `/Game/SV/Blueprints/BP_ChatMode` (`GameplayStatics.GetGameMode`)))
  (`/Game/SV/Blueprints/BP_ChatMode.GotMessageFromClient` _asbp_chat_mode (`KismetStringLibrary.Concat_StrStr` (`self.Userld`) ":" Msg)))

(event `self.ReceiveBeginPlay`
  ; 코멘트
  (if (not (`|EnumEquality` (`self.GetRemoteRole`) "ROLE_None"))
    (`KismetSystemLibrary.Delay` 0.5)
    (bind _foundwidgets (`WidgetBlueprintLibrary.GetAllWidgetsOfClass` "/Game/SV/UI/Widget_ChatWindow.Widget_ChatWindow_C"))
    (bind _output_get (set `self.Widget` (`|GetArrayItem` _foundwidgets)))
    (bind _aswidget_chat_window (cast `/Game/SV/UI/Widget_ChatWindow` _output_get))
    (add `/Game/SV/UI/Widget_ChatWindow.SetMessageToUserController` _aswidget_chat_window (`|CreateDelegate` :!event `OnSendMsgToServer`))))

(event `GotMessageFromClient`
  (params (Msg :type String :default "Msg"))
  ; NO
)

(fn `OnRep_As BP Chat Mode`)

(fn `UserConstructionScript`)